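; BP_GMB appears to be the game mode for a tower defense game, managing setup, waves and tower placement.
; BeginPlay enables mouse and touch-over interaction, builds a tower list from added Basic and Speed tower components, and creates the UI.
; CreateTower spawns a BP_TowerWrapper slightly offset from the selected tile and assigns it the chosen tower.
; StartGame and EndGame toggle the running flag; StartWave currently only prints each enemy class and its map value.
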(event `self.ReceiveBeginPlay`
  (`self.SetPlayerControllerVars`)
  (`self.MakeTowerList`)
  (`self.CreateUI`))

(event `StartGame`
  (params (WaveInfo :type "/Game/BP/WafeInfo Structure"))
  (`self.StartWave` WaveInfo)
  (set `self.GameRunning` true))

(event `EndGame`
  (set `self.GameRunning` false))

(fn `CreateTower`
  (params (NewTower :type "/Game/BP/Towers/BP_TowerData Object Reference"))
  (bind _selectedtile (`self.SelectedTile`))
  (`/Engine/EditorBlueprintResources/StandardMacros.IsValid` _selectedtile
    (:`Is Valid`
      (bind _returnvalue (`|SpawnActorFromClass` "/Game/BP/Towers/BP_TowerWrapper.BP_TowerWrapper_C" (`KismetMathLibrary.MakeTransform` (+ (.location (`self.GetTransform` _selectedtile)) (0.0 10.0 0.0)) (.rotation (`self.GetTransform` _selectedtile)) (.scale (`self.GetTransform` _selectedtile))) "Undefined" "OverrideRootScale" null null))
      (`/Game/BP/Towers/BP_TowerWrapper.SetTower` _returnvalue NewTower))))

(fn `CreateUI`
  (bind _returnvalue (`|CreateWidget` "/Game/BP/BP_UI.BP_UI_C"))
  (`UserWidget.AddToViewport` _returnvalue 0)
  (set `self.BP_UI` _returnvalue))

(fn `MakeTowerList`
  (bind _towerlist (`self.TowerList`))
  (bind _returnvalue (`AddComponent|NODE_AddBP_BasicTower-1`))
  (`KismetArrayLibrary.Array_Add` _towerlist _returnvalue)
  (bind _returnvalue_2 (`AddComponent|NODE_AddBP_SpeedTower-0`))
  (`KismetArrayLibrary.Array_Add` _towerlist _returnvalue_2))

(fn `SetPlayerControllerVars`
  (bind _returnvalue (`GameplayStatics.GetPlayerController` 0))
  (set `PlayerController.bShowMouseCursor` true _returnvalue)
  (set `PlayerController.bEnableClickEvents` true _returnvalue)
  (set `PlayerController.bEnableMouseOverEvents` true _returnvalue)
  (set `PlayerController.bEnableTouchOverEvents` true _returnvalue))

(fn `StartWave`
  (params (WaveInfo :type "/Game/BP/WafeInfo Structure"))
  (bind _enemies (break `/Game/BP/WafeInfo` WaveInfo))
  (bind _keys (`BlueprintMapLibrary.Map_Keys` _enemies))
  (for _array_element _keys
    (`KismetSystemLibrary.PrintString` (`KismetSystemLibrary.GetClassDisplayName` _array_element) true true (struct :`G` 1.0 :`B` 0.069008 :`A` 1.0))
    (`KismetSystemLibrary.PrintString` (`KismetStringLibrary.Conv_IntToString` (`BlueprintMapLibrary.Map_Find` _enemies _array_element)))))

(fn `UserConstructionScript`)