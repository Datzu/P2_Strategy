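; Base enemy actor that travels along the game's spline track from start to end.
; On Start it fetches the spline track from BP_GMB and plays a timeline whose play rate scales with EnemySpeed.
; Each update moves the actor to the lerped distance along the spline, and when the timeline finishes it prints a message and destroys itself.
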(event `Start`
  (bind _splinecomp (`/Game/BP/BP_Mark_line.SplineComp` (`self.SplineTrack`)))
  (bind _asbp_gmb (cast `/Game/BP/BP_GMB` (`GameplayStatics.GetGameMode`)))
  (bind _output_get (set `self.GMB` _asbp_gmb))
  (set `self.SplineTrack` (`/Game/BP/BP_GMB.SplineTrack` _output_get))
  (`/Engine/EditorBlueprintResources/StandardMacros.IsValid` (`self.SplineTrack`)
    (:`Is Valid`
      (`TimelineComponent.SetPlayRate` (`self.MoveTL`) (/ (`self.EnemySpeed`) 100.0))
      (bind (_direction _movetrack) (`Timeline|MoveTL`)
        (:`Update`
          (`self.K2_SetActorTransform` (`KismetMathLibrary.MakeTransform` (`SplineComponent.GetLocationAtDistanceAlongSpline` _splinecomp (`KismetMathLibrary.Lerp` 0.0 (`SplineComponent.GetSplineLength` _splinecomp) _movetrack) "World"))))
        (:`Finished`
          (`KismetSystemLibrary.PrintString` "Finished" true true (struct :`R` 1.0 :`B` 0.063568 :`A` 1.0))
          (`self.K2_DestroyActor`))))))

(fn `UserConstructionScript`)