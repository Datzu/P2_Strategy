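; BP_Tile is a selectable Paper2D tile that tints its sprite to show hover and selected states.
; A click resets the tile stored in the BP_GMB game mode's SelectedTile to its base color, then applies the click color and stores itself there, keeping selection exclusive.
; Cursor-over applies the hover color, and cursor exit restores either the click or base color depending on whether the tile is selected.
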(event `self.ReceiveBeginPlay`
  (bind _asbp_gmb (cast `/Game/BP/BP_GMB` (`GameplayStatics.GetGameMode`)))
  (set `self.GMB` _asbp_gmb))

(event `self.PaperSprite.OnClicked`
  (params (TouchedComponent :type "PrimitiveComponent Object Reference") (ButtonPressed :type "Key Structure"))
  (bind _selectedtile (`/Game/BP/BP_GMB.SelectedTile` (`self.GMB`)))
  (`/Engine/EditorBlueprintResources/StandardMacros.IsValid` _selectedtile
    (:`Is Valid`
      (`self.SetEndHoverColor` _selectedtile))
    (:`Is Not Valid`
      _))
  (`self.SetClickColor`)
  (set `/Game/BP/BP_GMB.SelectedTile` self (`self.GMB`)))

(event `self.PaperSprite.OnBeginCursorOver`
  (params (TouchedComponent :type "PrimitiveComponent Object Reference"))
  (`self.SetBeginHoverColor`))

(event `self.PaperSprite.OnEndCursorOver`
  (params (TouchedComponent :type "PrimitiveComponent Object Reference"))
  (if (== self (`/Game/BP/BP_GMB.SelectedTile` (`self.GMB`)))
    (`self.SetClickColor`)
    (else
      (`self.SetEndHoverColor`))))

(fn `SetBeginHoverColor`
  (`self.SetColor` (`self.HoverColor`)))

(fn `SetClickColor`
  (`self.SetColor` (`self.ClickColor`)))

(fn `SetColor`
  (params (NewColor :type "LinearColor Structure"))
  (`PaperSpriteComponent.SetSpriteColor` (`self.PaperSprite`) NewColor))

(fn `SetEndHoverColor`
  (`self.SetColor` (`self.BaseColor`)))

(fn `UserConstructionScript`)