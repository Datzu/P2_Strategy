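; BP_Mark_line is a spline track that draws a line of small mesh markers along its path and registers itself as the game mode's SplineTrack on BeginPlay.
; The construction script fills an instanced static mesh at even distances along the spline, spaced by the mesh's unscaled X extent plus an offset.
; Each instance is scaled down and unrotated, ignoring spline direction, and uses the disc material.
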(event `self.ReceiveBeginPlay`
  (bind _asbp_gmb (cast `/Game/BP/BP_GMB` (`GameplayStatics.GetGameMode`)))
  (set `/Game/BP/BP_GMB.SplineTrack` self _asbp_gmb))

(event `self.ReceiveTick`
  (params (DeltaSeconds :type "Float (single-precision)")))

(fn `UserConstructionScript`
  (locals (NumberOfInstances :type Integer :default 0))
  (bind (_min _max) (break `Box` (`StaticMesh.GetBoundingBox` (`self.PlacedMesh`))))
  (`StaticMeshComponent.SetStaticMesh` (`self.InstancedStaticMesh`) (`self.PlacedMesh`))
  (bind _output_get (set `self.Spacing` (+ (.x (- _max _min)) (`self.OffSet`))))
  (bind _output_get_2 (set `local.NumberOfInstances` (`KismetMathLibrary.FFloor` (/ (`SplineComponent.GetSplineLength` (`self.SplineComp`)) _output_get))))
  (for _index (range (+ _output_get_2 1))
    (`InstancedStaticMeshComponent.AddInstance` (`self.InstancedStaticMesh`) (`KismetMathLibrary.MakeTransform` (`SplineComponent.GetLocationAtDistanceAlongSpline` (`self.SplineComp`) (* _index (`self.Spacing`)) "Local") (struct) (0.1 0.1 0.1)) false)
    (`PrimitiveComponent.SetMaterial` (`self.InstancedStaticMesh`) 0 "/Engine/VREditor/UI/DiscMaterial.DiscMaterial")))